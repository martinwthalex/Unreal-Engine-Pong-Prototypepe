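; Pong paddle actor that slides its static mesh along a line between two marker actors, A and B.
; On BeginPlay it enables input from player controller 0 and adds the IMC_Player1 Enhanced Input mapping context.
; PlayerSelection decides whether the Player 1 or Player 2 movement action drives MoveRaquet.
; MoveRaquet scales input by Speed and delta time into a clamped 0–1 alpha that lerps the mesh position.
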(event `self.ReceiveBeginPlay`
  (bind _returnvalue (pcsubsystem `EnhancedInputLocalPlayerSubsystem` (`GameplayStatics.GetPlayerController` 0)))
  ;[1 1 1] CARGAR INPUT Y MAPPINGS
  (`/Engine/EditorBlueprintResources/StandardMacros.IsValid` _returnvalue
    (:`Is Valid`
      (`EnhancedInputSubsystemInterface.AddMappingContext` _returnvalue "/Game/Input/IMC_Player1.IMC_Player1" 0 (struct))
      (`self.EnableInput` (`GameplayStatics.GetPlayerController` 0)))))

(event `Move Raquet`
  (params (Quantity :type "Float (double-precision)"))
  ;[1 1 1] Interpola posicion del objeto entre A y B
  (set `self.C` (`KismetMathLibrary.FClamp` (+ (* Quantity (`GameplayStatics.GetWorldDeltaSeconds`) (`self.Speed`)) (`self.C`))))
  (`SceneComponent.K2_SetWorldLocation` (`self.StaticMeshComponent`) (`KismetMathLibrary.VLerp` (`self.K2_GetActorLocation` (`self.A`)) (`self.K2_GetActorLocation` (`self.B`)) (`self.C`)) false false))

(event `EnhancedInput|/Game/Input/Input_movement_Player1`
  (params (ActionValue :type "Float (double-precision)") (ElapsedSeconds :type "Float (double-precision)") (TriggeredSeconds :type "Float (double-precision)") (InputAction :type "InputAction Object Reference" :default "/Game/Input/Input_movement_Player1.Input_movement_Player1"))
  ;[1 1 1] Codigo que gestiona qué input se está pulsando
  (:`Triggered`
    (switch `/Game/Blueprints/Player_type` (`self.Player_selection`)
      (:`NewEnumerator0`
        (`self.Move Raquet` ActionValue)))))

(event `EnhancedInput|/Game/Input/Input_movement_Player2`
  (params (ActionValue :type "Float (double-precision)") (ElapsedSeconds :type "Float (double-precision)") (TriggeredSeconds :type "Float (double-precision)") (InputAction :type "InputAction Object Reference" :default "/Game/Input/Input_movement_Player2.Input_movement_Player2"))
  ;[1 1 1] Codigo que gestiona qué input se está pulsando
  (:`Triggered`
    (switch `/Game/Blueprints/Player_type` (`self.Player_selection`)
      (:`NewEnumerator1`
        (`self.Move Raquet` ActionValue)))))

(fn `UserConstructionScript`)