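; Physics-simulated bouncing ball that launches toward TargetInicial at BeginPlay and also adds a UI widget to the viewport.
; Each hit increments a bounce counter and reflects the normalized direction using the hit's NormalImpulse.
; Four chained Watch checks, one per heading quadrant, nudge directions near ±90° away from that axis to avoid sideways bounces.
; The direction times Velocity then overwrites the mesh's linear velocity, while overlaps only print the other actor's name.
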(event `self.ReceiveBeginPlay`
  ;[1 1 1] Iniciar
  (`PrimitiveComponent.SetSimulatePhysics` (`self.StaticMeshComponent`) true)
  (`self.Calculate Initial Direction`)
  (`self.Calculate Impulse`)
  ;[1 1 1] UI CANVAS con widgets
  (bind _returnvalue (`|CreateWidget` "/Game/Blueprints/My_Widget_BP.My_Widget_BP_C" (`GameplayStatics.GetPlayerController` 0)))
  (`UserWidget.AddToViewport` _returnvalue 0))

(event `Calculate Initial Direction`
  ;[1 1 1] Set direction
  (set `self.direction` (`KismetMathLibrary.Normal` (- (`self.K2_GetActorLocation` (`self.Target Inicial`)) (`self.K2_GetActorLocation` self)))))

(event `Calculate Impulse`
  ;[1 1 1] Set Impulse
  (`PrimitiveComponent.SetPhysicsLinearVelocity` (`self.StaticMeshComponent`) (* (`self.direction`) (`self.Velocity`)) false "None"))

(event `self.StaticMeshComponent.OnComponentHit`
  (params (HitComponent :type "PrimitiveComponent Object Reference") (OtherActor :type "Actor Object Reference") (OtherComp :type "PrimitiveComponent Object Reference") (NormalImpulse :type "Vector Structure") (Hit :type "HitResult Structure (by ref)"))
  ;[1 1 1] Rebota contra la pared, recalculamos direccion con el vactor reflection
  (`/Engine/EditorBlueprintResources/StandardMacros.IncrementInt` (`self.num_rebounds`)
    (:`  `
      (bind _output_get (set `self.direction` (`KismetMathLibrary.Normal` (`KismetMathLibrary.GetReflectionVector` (`self.direction`) NormalImpulse))))
      (bind _returnvalue (`KismetMathLibrary.RadiansToDegrees` (`KismetMathLibrary.Vector_HeadingAngle` _output_get)))
      ;[1 1 1] Comprueba los ángulos de rebote y los modifica si fuese necesario
      (if (and (> _returnvalue (`self.forward_MAX`)) (< _returnvalue 90.0))
        (bind _output_get_2 (set `self.direction` (`KismetMathLibrary.RotateAngleAxis` (`self.direction`) -10.0 (0.0 0.0 1.0)))))
      (bind _returnvalue_2 (`KismetMathLibrary.RadiansToDegrees` (`KismetMathLibrary.Vector_HeadingAngle` _output_get_2)))
      (if (and (< _returnvalue_2 (`self.backward_MAX`)) (> _returnvalue_2 90.0))
        (bind _output_get_3 (set `self.direction` (`KismetMathLibrary.RotateAngleAxis` (`self.direction`) 10.0 (0.0 0.0 1.0)))))
      (bind _returnvalue_3 (`KismetMathLibrary.RadiansToDegrees` (`KismetMathLibrary.Vector_HeadingAngle` _output_get_3)))
      (if (and (< _returnvalue_3 (`self.forward_MIN`)) (> _returnvalue_3 -90.0))
        (bind _output_get_4 (set `self.direction` (`KismetMathLibrary.RotateAngleAxis` (`self.direction`) 10.0 (0.0 0.0 1.0))))
        (else
          (bind _returnvalue_4 (`KismetMathLibrary.RadiansToDegrees` (`KismetMathLibrary.Vector_HeadingAngle` _output_get_4)))
          (if (and (> _returnvalue_4 (`self.backward_MIN`)) (< _returnvalue_4 -90.0))
            (set `self.direction` (`KismetMathLibrary.RotateAngleAxis` (`self.direction`) -10.0 (0.0 0.0 1.0))))))
      (`self.Calculate Impulse`))))

(event `self.StaticMeshComponent.OnComponentBeginOverlap`
  (params (OverlappedComponent :type "PrimitiveComponent Object Reference") (OtherActor :type "Actor Object Reference") (OtherComp :type "PrimitiveComponent Object Reference") (OtherBodyIndex :type Integer) (bFromSweep :type Boolean) (SweepResult :type "HitResult Structure (by ref)"))
  (`KismetSystemLibrary.PrintString` (`KismetSystemLibrary.GetDisplayName` OtherActor) true true (struct :`R` 0.879707 :`G` 1.0 :`A` 1.0)))

(fn `UserConstructionScript`)